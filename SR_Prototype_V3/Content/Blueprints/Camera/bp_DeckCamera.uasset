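; A ship deck camera Blueprint that shows a live 2D capture of its deck in the ship's UI.
; AddTextureTarget assigns a render target to the capture component and stores the matching camera material.
; It then creates a deck view widget labeled with camera number and deck name, using that material as the image.
; The widget joins the main widget's deck view box and the ship's widget list.
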(event Custom|AddTextureTarget
  (params (RenderTarget :type Texture%20Render%20Target%202D%20Object%20Reference) (CamMat :type Material%20Object%20Reference))
  (bind _bp_ship (Variables|Default|Getbp_ship))
  (Variables|/Script/Engine.SceneCaptureComponent2D|SetTextureTarget (Variables|DecalActor|GetCaptureComponent2D) RenderTarget)
  (bind _output_get (Variables|Default|SetCameraMat CamMat))
  (bind _returnvalue (UserInterface|CreateWidget "/Game/Blueprints/Widgets/w_Deckview.w_Deckview_C" 0 (Variables|Default|Getbp_ship) self))
  (Variables|/Game/Blueprints/Widgets/w_Deckview.w_Deckview_C|SetMyCameraNumber _returnvalue (Utilities|Text|ToText(Integer) (Variables|Default|GetCameraNumber)))
  (Rendering|Components|TextRender|SetText (Variables|/Game/Blueprints/Widgets/w_Deckview.w_Deckview_C|GetDeckName _returnvalue) (Utilities|Struct|Breaks_FloorInfo (Variables|/Game/Blueprints/Ship/bp_Deck.bp_Deck_C|GetDeckInfo (Variables|Default|GetMyDeck))))
  (Class|Image|SetBrushfromMaterial (Variables|/Game/Blueprints/Widgets/w_Deckview.w_Deckview_C|GetCamera_View _returnvalue) _output_get)
  (Class|VerticalBox|AddChildtoVerticalBox (Variables|/Game/Blueprints/Widgets/w_deckViewBox.w_deckViewBox_C|GetDeckViewBox (Variables|/Game/Blueprints/Widgets/w_Main.w_Main_C|Getw_deckViewBox (Variables|/Game/Blueprints/Ship/bp_Ship.bp_Ship_C|GetMainWidget _bp_ship))) _returnvalue)
  (Variables|Default|SetMyDeckViewWidget _returnvalue)
  (Utilities|Array|Add (Variables|/Game/Blueprints/Ship/bp_Ship.bp_Ship_C|GetDeckViewUIWidgets _bp_ship) _returnvalue))

(fn ConstructionScript)