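; bp_Sensor is a ship sensor Blueprint that holds the most recent reading passed to it.
; UpdateInformation overwrites the stored temperature, time, date, voltage and RSSI, then passes the tag ID to UpdateTagIDs, which keeps a list of unique IDs seen.
; Readings are not stored per tag, and the event graph and construction script are empty, so updates rely on external calls.
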(event EventBeginPlay)

(event Collision|EventActorBeginOverlap
  (params (OtherActor :type Actor%20Object%20Reference)))

(event EventTick
  (params (DeltaSeconds :type Float%20%28single-precision%29)))

(fn ConstructionScript)

(fn UpdateInformation
  (params (TagID :type String) (Temp :type String) (Time :type String) (Date :type String) (Volt :type String) (RSSI :type String))
  (Variables|Default|SetTime Time)
  (Variables|Default|SetDate Date)
  (Variables|Default|SetRSSI RSSI)
  (Variables|Default|SetVolt Volt)
  (Variables|Default|SetTemperature Temp)
  (CallFunction|UpdateTagID's TagID))

(fn UpdateTagID's
  (params (TagID :type String))
  (bind _tagid_s (Variables|Default|GetTagID's))
  (if (not (Utilities|Array|ContainsItem _tagid_s TagID))
    (Utilities|Array|AddUnique _tagid_s TagID)))