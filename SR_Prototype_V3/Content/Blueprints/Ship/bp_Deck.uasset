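; bp_Deck is a ship deck actor that displays a single deck's name and image.
; On BeginPlay it caches its world location as DeckPosition.
; SetDeckInfo stores the deck data, writes the name to the FloorNamePreview text and applies the 2048 deck image to the floor mesh through a dynamic instance of M_Deck.
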(event EventBeginPlay
  (Variables|Default|SetDeckPosition (Transformation|GetActorLocation)))

(event Collision|EventActorBeginOverlap
  (params (OtherActor :type Actor%20Object%20Reference)))

(event EventTick
  (params (DeltaSeconds :type Float%20%28single-precision%29)))

(fn ConstructionScript)

(fn SetDeckInfo
  (params (DeckInfo :type S%20Floor%20Info%20Structure))
  (bind _output_get (Variables|Default|SetDeckInfo DeckInfo))
  (Rendering|Components|TextRender|SetText (Variables|Default|GetFloorName_Preview) (.DeckName (Utilities|Struct|Breaks_FloorInfo _output_get)))
  (bind _returnvalue (Rendering|Material|CreateDynamicMaterialInstance (Variables|Default|GetFloorMesh) 0 "/Game/Materials/m_Deck.m_Deck" :!class /Script/Engine.PrimitiveComponent))
  (bind _output_get_2 (Variables|Default|SetDeckMaterial _returnvalue))
  (Rendering|Material|SetTextureParameterValue _output_get_2 "DeckImage" (.DeckImage2048 (Utilities|Struct|Breaks_FloorInfo _output_get))))