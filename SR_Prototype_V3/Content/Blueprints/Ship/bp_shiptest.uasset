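; Test ship Blueprint that creates the main UI and a set of deck-view cameras at BeginPlay.
; It gathers CameraPosPoint actors as deck markers, then adds a W_Main widget holding a reference to the ship.
; CreateDeckViewCameras caps the camera count to the marker count and spawns Bp_deckCamera at each marker's XY, using its ZoominValue as height.
; Each camera receives a ship reference, number, render target and material from index-matched arrays.
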(event EventBeginPlay
  (bind _outactors (Actor|GetAllActorsOfClass "/Game/Blueprints/Camera/CameraPosPoint.CameraPosPoint_C"))
  (Variables|Default|SetDeckActors _outactors)
  (bind _returnvalue (UserInterface|CreateWidget "/Game/Blueprints/Widgets/w_Main.w_Main_C"))
  (Variables|Default|SetMainWidget _returnvalue)
  (Variables|/Game/Blueprints/Widgets/w_Main.w_Main_C|SetBp_Ship _returnvalue self)
  (UserInterface|Viewport|AddtoViewport _returnvalue 0)
  (CallFunction|CreateDeckViewCameras))

(event Collision|EventActorBeginOverlap
  (params (OtherActor :type Actor%20Object%20Reference)))

(event EventTick
  (params (DeltaSeconds :type Float%20%28single-precision%29)))

(fn ConstructionScript)

(fn CreateDeckViewCameras
  (bind _deckactors (Variables|Default|GetDeckActors))
  (bind _returnvalue (Utilities|Array|Length _deckactors))
  (if (< _returnvalue (Variables|Default|GetNumberOfCameras))
    (Variables|Default|SetNumberOfCameras _returnvalue))
  (for _index (range (Variables|Default|GetFirstCameraIndex) (Variables|Default|GetNumberOfCameras))
    (bind _returnvalue_2 (Game|SpawnActorfromClass "/Game/Blueprints/Camera/bp_DeckCamera.bp_deckCamera_C" (Math|Transform|MakeTransform (Math|Vector|MakeVector (.X (Math|Vector|BreakVector (Transformation|GetActorLocation (Utilities|Array|Get(acopy) (Variables|Default|GetDeckActors) (- _index 1))))) (.Y (Math|Vector|BreakVector (Transformation|GetActorLocation (Utilities|Array|Get(acopy) (Variables|Default|GetDeckActors) (- _index 1))))) (Math|Conversions|ToFloat(Integer) (Variables|/Game/Blueprints/Camera/CameraPosPoint.CameraPosPoint_C|GetZoominValue (Utilities|Array|Get(acopy) _deckactors (- _index 1))))) "0, 0, 0" "1,1,1") "Undefined" 0 0))
    (Variables|/Game/Blueprints/Camera/bp_DeckCamera.bp_deckCamera_C|Setbp_ship _returnvalue_2 self)
    (Variables|/Game/Blueprints/Camera/bp_DeckCamera.bp_deckCamera_C|SetCameraNumber _returnvalue_2 _index)
    (Default|AddTextureTarget _returnvalue_2 (Utilities|Array|Get(acopy) (Variables|Default|GetCameraTextureTargets) (- _index 1)) (Utilities|Array|Get(acopy) (Variables|Default|GetCameraMaterials) (- _index 1)))))