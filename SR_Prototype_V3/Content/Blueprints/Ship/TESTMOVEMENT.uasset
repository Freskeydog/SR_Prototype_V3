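; TESTMOVEMENT is a test asset in the Ship folder that registers itself as one of the ship's pawns.
; On BeginPlay it adds itself uniquely to BpShip's AllPawns array, then waits briefly before refreshing the passenger display in the main widget's ship info panel.
; Tick is empty, and a node that would show TagID on a text render is unconnected, so no movement logic is present.
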(event EventBeginPlay
  (Utilities|Array|AddUnique (Variables|/Game/Blueprints/Ship/bp_Ship.bp_Ship_C|GetAllPawns (Variables|Default|Getbp_ship)) self)
  (Utilities|FlowControl|Delay 0.2)
  (Default|UpdatePassenger (Variables|/Game/Blueprints/Widgets/w_Main.w_Main_C|Getw_shipInfo (Variables|/Game/Blueprints/Ship/bp_Ship.bp_Ship_C|GetMainWidget (Variables|Default|Getbp_ship)))))

(event EventTick
  (params (DeltaSeconds :type Float%20%28single-precision%29)))

(fn ConstructionScript)