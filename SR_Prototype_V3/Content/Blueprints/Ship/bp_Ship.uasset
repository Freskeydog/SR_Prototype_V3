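; Ship actor that builds a deck layout from data and manages a multi-camera deck monitoring view.
; The construction script spawns offset bp_Deck child actors; BeginPlay creates the main widget, spawns render-target cameras above the first decks and removes unused muster stations.
; Deck buttons move an inactive camera to the chosen deck, or cycle round-robin through cameras, updating labels and warning/emergency name colors.
; Removing a view deactivates its camera for reuse.
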(event EventBeginPlay
  (bind _returnvalue (UserInterface|CreateWidget "/Game/Blueprints/Widgets/w_Main.w_Main_C"))
  (Variables|UI/HUD|SetMainWidget _returnvalue)
  (Variables|/Game/Blueprints/Widgets/w_Main.w_Main_C|SetBp_Ship _returnvalue self)
  (UserInterface|Viewport|AddtoViewport _returnvalue 0)
  (Utilities|FlowControl|Delay 0.3)
  (CallFunction|CreateDeckViewCameras)
  (for _array_element (Variables|Deck|GetDeckActors)
    (if (not (Utilities|Struct|Breaks_FloorInfo (Variables|/Game/Blueprints/Ship/bp_Deck.bp_Deck_C|GetDeckInfo _array_element)))
      (Default|DestroyMusterStation _array_element))))

(fn ConstructionScript
  (bind _decks (Variables|Deck|GetDecks))
  (bind (_decks_2 _distancebetweendecks _deckscale _namesize _namelocation) (Utilities|Struct|Breaks_DeckSetup _decks))
  (Utilities|Array|Clear (Variables|Deck|GetDeckActors))
  (for (_array_element _array_index) _decks_2
    (bind _structout (Utilities|Struct|Setmembersins_FloorInfo _array_element _array_index))
    (CallFunction|CreateNewDeck _structout _distancebetweendecks _deckscale _namesize _namelocation (LocalVariables|GetDeckStartingPos))
    (LocalVariables|SetDeckStartingPos (+ (LocalVariables|GetDeckStartingPos) (Math|Vector|MakeVector 0.0 _distancebetweendecks 0.0)))))

(fn CreateNewDeck
  (params (DeckINfo :type S%20Floor%20Info%20Structure) (DistanceBetweenDeck :type Float%20%28single-precision%29) (DeckScale :type Float%20%28single-precision%29) (NameSize :type Float%20%28single-precision%29) (NameLocation :type Vector) (DeckPos :type Vector))
  (bind (_staircasepos _hasmuster_ _musterpos _mustersize) (Utilities|Struct|Breaks_FloorInfo DeckINfo))
  (bind _returnvalue (AddComponent|AddChildActorComponent false (Math|Transform|MakeTransform DeckPos "0, 0, 0" (Math|Conversions|ToVector(Float) DeckScale))))
  (bind _asbp_deck (Utilities|Casting|CastTobp_Deck (Variables|/Script/Engine.ChildActorComponent|GetChildActor _returnvalue)))
  (Variables|/Game/Blueprints/Ship/bp_Deck.bp_Deck_C|SetDeckInfo _asbp_deck DeckINfo)
  (Variables|/Game/Blueprints/Ship/bp_Deck.bp_Deck_C|Setbp_ship _asbp_deck self)
  (Utilities|Array|Add (Variables|Deck|GetDeckActors) _asbp_deck)
  (Default|SetDeckInfo _asbp_deck DeckINfo)
  (Rendering|Components|TextRender|SetWorldSize (Variables|/Game/Blueprints/Ship/bp_Deck.bp_Deck_C|GetFloorName_Preview _asbp_deck) NameSize)
  (Transformation|SetRelativeLocation (Variables|/Game/Blueprints/Ship/bp_Deck.bp_Deck_C|GetFloorName_Preview _asbp_deck) NameLocation false false)
  (Transformation|SetRelativeLocation (Variables|/Game/Blueprints/Ship/bp_Deck.bp_Deck_C|GetStairCaseCollision _asbp_deck) _staircasepos false false)
  (Components|Box|SetBoxExtent (Variables|/Game/Blueprints/Ship/bp_Deck.bp_Deck_C|GetMusterCollision _asbp_deck) _mustersize true)
  (Transformation|SetRelativeLocation (Variables|/Game/Blueprints/Ship/bp_Deck.bp_Deck_C|GetMusterCollision _asbp_deck) _musterpos false false))

(fn CreateDeckViewCameras
  (bind _decks (Variables|Deck|GetDecks))
  (bind _decks_2 (Utilities|Struct|Breaks_DeckSetup _decks))
  (bind _returnvalue (Utilities|Array|Length _decks_2))
  (if (< _returnvalue (Variables|Camera|GetNumberOfCameras))
    (Variables|Camera|SetNumberOfCameras _returnvalue))
  (for _index (range (LocalVariables|GetFirstCamIndex) (Variables|Camera|GetNumberOfCameras))
    (Variables|/Game/Blueprints/Ship/bp_Deck.bp_Deck_C|SetSelected? (Utilities|Array|Get(acopy) (Variables|Deck|GetDeckActors) (- _index 1)) true)
    (bind _returnvalue_2 (Game|SpawnActorfromClass "/Game/Blueprints/Camera/bp_DeckCamera.bp_deckCamera_C" (Math|Transform|MakeTransform (Math|Vector|MakeVector (.X (Math|Vector|BreakVector (Variables|/Game/Blueprints/Ship/bp_Deck.bp_Deck_C|GetDeckPosition (Utilities|Array|Get(acopy) (Variables|Deck|GetDeckActors) (- _index 1))))) (.Y (Math|Vector|BreakVector (Variables|/Game/Blueprints/Ship/bp_Deck.bp_Deck_C|GetDeckPosition (Utilities|Array|Get(acopy) (Variables|Deck|GetDeckActors) (- _index 1))))) 1.7e+03) "0,0.000000, 0" "1,1,1") "Undefined" 0 0))
    (Variables|/Game/Blueprints/Camera/bp_DeckCamera.bp_deckCamera_C|SetCameraNumber _returnvalue_2 _index)
    (bind _output_get (Variables|/Game/Blueprints/Camera/bp_DeckCamera.bp_deckCamera_C|SetMyDeck _returnvalue_2 (Utilities|Array|Get(acopy) (Variables|Deck|GetDeckActors) (- _index 1))))
    (Variables|/Game/Blueprints/Widgets/w_DeckButton.w_DeckButton_C|SetMyCurrentCamera (Variables|/Game/Blueprints/Ship/bp_Deck.bp_Deck_C|GetMyButton _output_get) _returnvalue_2)
    (Variables|/Game/Blueprints/Ship/bp_Deck.bp_Deck_C|SetMyCamera _output_get _returnvalue_2)
    (Variables|/Game/Blueprints/Camera/bp_DeckCamera.bp_deckCamera_C|Setbp_ship _returnvalue_2 self)
    (Default|AddTextureTarget _returnvalue_2 (Utilities|Array|Get(acopy) (Variables|Camera|GetCameraTextureTargets) (- _index 1)) (Utilities|Array|Get(acopy) (Variables|Camera|GetCameraMaterials) (- _index 1)))
    (Utilities|Array|Add (Variables|Camera|GetDeckCameraActors) _returnvalue_2)
    (Variables|/Game/Blueprints/Camera/bp_DeckCamera.bp_deckCamera_C|SetActive? _returnvalue_2 true)
    (Widget|SetVisibility (Variables|/Game/Blueprints/Widgets/w_DeckButton.w_DeckButton_C|GetDeckRemove_Button (Variables|/Game/Blueprints/Ship/bp_Deck.bp_Deck_C|GetMyButton _output_get)) "Visible")
    (Variables|/Game/Blueprints/Widgets/w_DeckButton.w_DeckButton_C|SetCameraIndex (Variables|/Game/Blueprints/Ship/bp_Deck.bp_Deck_C|GetMyButton _output_get) (Utilities|Text|ToText(Integer) _index))))

(fn ChangeDeckView
  (params (DeckButton :type W%20Deck%20Button%20Object%20Reference))
  (bind _deckcameraactors (Variables|Camera|GetDeckCameraActors))
  (bind _output_get (LocalVariables|SetButtonPressed DeckButton))
  (if (not (Variables|/Game/Blueprints/Ship/bp_Deck.bp_Deck_C|GetSelected? (Variables|/Game/Blueprints/Widgets/w_DeckButton.w_DeckButton_C|GetDeckRef _output_get)))
    (for _array_element (Variables|Camera|GetDeckCameraActors)
      (if (not (Variables|/Game/Blueprints/Camera/bp_DeckCamera.bp_deckCamera_C|GetActive? _array_element))
        (Utilities|FlowControl|DoOnce false
          (:Completed
            (LocalVariables|SetInactiveCamera _array_element)
            (Variables|Camera|SetCameraToChange 0)))))
    (Utilities|IsValid (LocalVariables|GetInactiveCamera)
      (:Is%20Valid
        (Variables|/Game/Blueprints/Ship/bp_Deck.bp_Deck_C|SetSelected? (Variables|/Game/Blueprints/Camera/bp_DeckCamera.bp_deckCamera_C|GetMyDeck (LocalVariables|GetInactiveCamera)) false)
        (Widget|SetVisibility (Variables|/Game/Blueprints/Widgets/w_DeckButton.w_DeckButton_C|GetDeckRemove_Button (Variables|/Game/Blueprints/Ship/bp_Deck.bp_Deck_C|GetMyButton (Variables|/Game/Blueprints/Camera/bp_DeckCamera.bp_deckCamera_C|GetMyDeck (LocalVariables|GetInactiveCamera)))) "Hidden")
        (Transformation|SetActorLocation (LocalVariables|GetInactiveCamera) (Math|Vector|MakeVector (.X (Math|Vector|BreakVector (Variables|/Game/Blueprints/Ship/bp_Deck.bp_Deck_C|GetDeckPosition (Variables|/Game/Blueprints/Widgets/w_DeckButton.w_DeckButton_C|GetDeckRef (LocalVariables|GetButtonPressed))))) (.Y (Math|Vector|BreakVector (Variables|/Game/Blueprints/Ship/bp_Deck.bp_Deck_C|GetDeckPosition (Variables|/Game/Blueprints/Widgets/w_DeckButton.w_DeckButton_C|GetDeckRef (LocalVariables|GetButtonPressed))))) 1.7e+03) false false)
        (Variables|/Game/Blueprints/Widgets/w_DeckButton.w_DeckButton_C|SetMyCurrentCamera (LocalVariables|GetButtonPressed) (LocalVariables|GetInactiveCamera))
        (bind _output_get_2 (Variables|/Game/Blueprints/Camera/bp_DeckCamera.bp_deckCamera_C|SetMyDeck (LocalVariables|GetInactiveCamera) (Variables|/Game/Blueprints/Widgets/w_DeckButton.w_DeckButton_C|GetDeckRef (LocalVariables|GetButtonPressed))))
        (Widget|SetVisibility (Variables|/Game/Blueprints/Widgets/w_DeckButton.w_DeckButton_C|GetDeckRemove_Button (LocalVariables|GetButtonPressed)) "Visible")
        (Widget|SetVisibility (Variables|/Game/Blueprints/Camera/bp_DeckCamera.bp_deckCamera_C|GetMyDeckViewWidget (LocalVariables|GetInactiveCamera)) "Visible")
        (Rendering|Components|TextRender|SetText (Variables|/Game/Blueprints/Widgets/w_Deckview.w_Deckview_C|GetDeckName (Variables|/Game/Blueprints/Camera/bp_DeckCamera.bp_deckCamera_C|GetMyDeckViewWidget (LocalVariables|GetInactiveCamera))) (Utilities|Struct|Breaks_FloorInfo (Variables|/Game/Blueprints/Ship/bp_Deck.bp_Deck_C|GetDeckInfo _output_get_2)))
        (Variables|/Game/Blueprints/Camera/bp_DeckCamera.bp_deckCamera_C|SetActive? (LocalVariables|GetInactiveCamera) true)
        (Variables|/Game/Blueprints/Ship/bp_Deck.bp_Deck_C|SetSelected? (Variables|/Game/Blueprints/Widgets/w_DeckButton.w_DeckButton_C|GetDeckRef (LocalVariables|GetButtonPressed)) true)
        (Variables|/Game/Blueprints/Widgets/w_DeckButton.w_DeckButton_C|SetCameraIndex (LocalVariables|GetButtonPressed) (Utilities|Text|ToText(Integer) (Variables|/Game/Blueprints/Camera/bp_DeckCamera.bp_deckCamera_C|GetCameraNumber (LocalVariables|GetInactiveCamera))))
        (if (Variables|/Game/Blueprints/Ship/bp_Deck.bp_Deck_C|GetWarning? _output_get_2)
          (Default|SetNameYellow (Variables|/Game/Blueprints/Camera/bp_DeckCamera.bp_deckCamera_C|GetMyDeckViewWidget (LocalVariables|GetInactiveCamera)))
          (elif (Variables|/Game/Blueprints/Ship/bp_Deck.bp_Deck_C|GetEmergency? _output_get_2)
            (Default|SetNameRed (Variables|/Game/Blueprints/Camera/bp_DeckCamera.bp_deckCamera_C|GetMyDeckViewWidget (LocalVariables|GetInactiveCamera)))
            (else
              (Default|SetNameNormal (Variables|/Game/Blueprints/Camera/bp_DeckCamera.bp_deckCamera_C|GetMyDeckViewWidget (LocalVariables|GetInactiveCamera)))))))
      (:Is%20Not%20Valid
        (Variables|/Game/Blueprints/Ship/bp_Deck.bp_Deck_C|SetSelected? (Variables|/Game/Blueprints/Camera/bp_DeckCamera.bp_deckCamera_C|GetMyDeck (Utilities|Array|Get(acopy) (Variables|Camera|GetDeckCameraActors) (Variables|Camera|GetCameraToChange))) false)
        (Widget|SetVisibility (Variables|/Game/Blueprints/Widgets/w_DeckButton.w_DeckButton_C|GetDeckRemove_Button (Variables|/Game/Blueprints/Ship/bp_Deck.bp_Deck_C|GetMyButton (Variables|/Game/Blueprints/Camera/bp_DeckCamera.bp_deckCamera_C|GetMyDeck (Utilities|Array|Get(acopy) (Variables|Camera|GetDeckCameraActors) (Variables|Camera|GetCameraToChange))))) "Hidden")
        (Transformation|SetActorLocation (Utilities|Array|Get(acopy) (Variables|Camera|GetDeckCameraActors) (Variables|Camera|GetCameraToChange)) (Math|Vector|MakeVector (.X (Math|Vector|BreakVector (Variables|/Game/Blueprints/Ship/bp_Deck.bp_Deck_C|GetDeckPosition (Variables|/Game/Blueprints/Widgets/w_DeckButton.w_DeckButton_C|GetDeckRef (LocalVariables|GetButtonPressed))))) (.Y (Math|Vector|BreakVector (Variables|/Game/Blueprints/Ship/bp_Deck.bp_Deck_C|GetDeckPosition (Variables|/Game/Blueprints/Widgets/w_DeckButton.w_DeckButton_C|GetDeckRef (LocalVariables|GetButtonPressed))))) 1.7e+03) false false)
        (bind _output_get_3 (Variables|/Game/Blueprints/Widgets/w_DeckButton.w_DeckButton_C|SetMyCurrentCamera (LocalVariables|GetButtonPressed) (Utilities|Array|Get(acopy) (Variables|Camera|GetDeckCameraActors) (Variables|Camera|GetCameraToChange))))
        (Variables|/Game/Blueprints/Ship/bp_Deck.bp_Deck_C|SetSelected? (Variables|/Game/Blueprints/Widgets/w_DeckButton.w_DeckButton_C|GetDeckRef (LocalVariables|GetButtonPressed)) true)
        (Widget|SetVisibility (Variables|/Game/Blueprints/Widgets/w_DeckButton.w_DeckButton_C|GetDeckRemove_Button (LocalVariables|GetButtonPressed)) "Visible")
        (bind _output_get_4 (Variables|/Game/Blueprints/Camera/bp_DeckCamera.bp_deckCamera_C|SetMyDeck (Utilities|Array|Get(acopy) (Variables|Camera|GetDeckCameraActors) (Variables|Camera|GetCameraToChange)) (Variables|/Game/Blueprints/Widgets/w_DeckButton.w_DeckButton_C|GetDeckRef (LocalVariables|GetButtonPressed))))
        (Variables|/Game/Blueprints/Widgets/w_DeckButton.w_DeckButton_C|SetCameraIndex (LocalVariables|GetButtonPressed) (Utilities|Text|ToText(Integer) (Variables|/Game/Blueprints/Camera/bp_DeckCamera.bp_deckCamera_C|GetCameraNumber (Utilities|Array|Get(acopy) (Variables|Camera|GetDeckCameraActors) (Variables|Camera|GetCameraToChange)))))
        (Rendering|Components|TextRender|SetText (Variables|/Game/Blueprints/Widgets/w_Deckview.w_Deckview_C|GetDeckName (Variables|/Game/Blueprints/Camera/bp_DeckCamera.bp_deckCamera_C|GetMyDeckViewWidget _output_get_3)) (Utilities|Struct|Breaks_FloorInfo (Variables|/Game/Blueprints/Ship/bp_Deck.bp_Deck_C|GetDeckInfo _output_get_4)))
        (if (Variables|/Game/Blueprints/Ship/bp_Deck.bp_Deck_C|GetWarning? _output_get_4)
          (Default|SetNameYellow (Variables|/Game/Blueprints/Camera/bp_DeckCamera.bp_deckCamera_C|GetMyDeckViewWidget _output_get_3))
          (elif (Variables|/Game/Blueprints/Ship/bp_Deck.bp_Deck_C|GetEmergency? _output_get_4)
            (Default|SetNameRed (Variables|/Game/Blueprints/Camera/bp_DeckCamera.bp_deckCamera_C|GetMyDeckViewWidget _output_get_3))
            (else
              (Default|SetNameNormal (Variables|/Game/Blueprints/Camera/bp_DeckCamera.bp_deckCamera_C|GetMyDeckViewWidget _output_get_3)))))
        (if (>= (Variables|Camera|GetCameraToChange) (Utilities|Array|LastIndex _deckcameraactors))
          (Variables|Camera|SetCameraToChange 0)
          (else
            (Variables|Camera|SetCameraToChange (+ (Utilities|Array|FindItem _deckcameraactors (Utilities|Array|Get(acopy) (Variables|Camera|GetDeckCameraActors) (Variables|Camera|GetCameraToChange))) 1))))))))

(fn RemoveDeckView
  (params (DeckButton :type W%20Deck%20Button%20Object%20Reference))
  (Variables|/Game/Blueprints/Camera/bp_DeckCamera.bp_deckCamera_C|SetActive? (Variables|/Game/Blueprints/Widgets/w_DeckButton.w_DeckButton_C|GetMyCurrentCamera DeckButton) false)
  (Widget|SetVisibility (Variables|/Game/Blueprints/Camera/bp_DeckCamera.bp_deckCamera_C|GetMyDeckViewWidget (Variables|/Game/Blueprints/Widgets/w_DeckButton.w_DeckButton_C|GetMyCurrentCamera DeckButton)) "Hidden")
  (Variables|/Game/Blueprints/Widgets/w_DeckButton.w_DeckButton_C|SetMyCurrentCamera DeckButton 0)
  (Widget|SetVisibility (Variables|/Game/Blueprints/Widgets/w_DeckButton.w_DeckButton_C|GetDeckRemove_Button DeckButton) "Hidden")
  (Variables|/Game/Blueprints/Ship/bp_Deck.bp_Deck_C|SetSelected? (Variables|/Game/Blueprints/Widgets/w_DeckButton.w_DeckButton_C|GetDeckRef DeckButton) false))