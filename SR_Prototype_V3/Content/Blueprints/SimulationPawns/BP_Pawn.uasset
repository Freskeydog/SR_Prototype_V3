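; BP_Pawn is a simulation pawn that walks a looping route through an array of target points.
; On BeginPlay it caches its BP_Pawn_Controller and uses SimpleMoveToActor to head for the point at the current index.
; The OverlappedOnePoint event advances the index, wrapping to zero after the last point, and issues the next move.
; Despite its name, SearchForClosestPoint follows array order and does no distance check.
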(event Custom|SearchForClosestPoint
  (AI|Navigation|SimpleMovetoActor (Variables|Default|GetPawnControllerRef) (Utilities|Array|Get(acopy) (Variables|Default|GetTargetPointsArray) (Variables|Default|GetIndexToWalkTo))))

(event Custom|OverlappedOnePoint
  (bind _output_get (Variables|Default|SetIndexToWalkTo (+ (Variables|Default|GetIndexToWalkTo) 1)))
  (if (> _output_get (- (Utilities|Array|Length (Variables|Default|GetTargetPointsArray)) 1))
    (Variables|Default|SetIndexToWalkTo 0)
    (CallFunction|SearchforClosestPoint)
    (else
      (CallFunction|SearchforClosestPoint))))

(event EventBeginPlay
  (bind _asbp_pawn_controller (Utilities|Casting|CastToBP_Pawn_Controller (Pawn|GetController)))
  (Variables|Default|SetPawnControllerRef _asbp_pawn_controller)
  (CallFunction|SearchforClosestPoint))

(fn ConstructionScript)