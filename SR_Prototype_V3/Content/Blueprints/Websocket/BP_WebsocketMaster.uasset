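; Master websocket actor that receives ScanReach tag data and drives tag pawns in the level through their sensors.
; In Websocket mode it connects shortly after BeginPlay, sends an interval setting, reconnects on errors and supports switching between live and echo servers.
; Incoming JSON becomes a WebsocketTest object, whose TagID finds or spawns a TESTMOVEMENT pawn.
; Sensors with a matching SensorID store the data and search for and move that tag.
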(event Custom|WebSocketConnected
  (Development|PrintString (Utilities|String|Append "Connected To: " (Variables|Default|GetServerToConnectTo)))
  (EventDispatchers|AssignOnReceiveData (stale Custom|ConnectToServer _output_get) (delegate Custom|WebSocketRecieve%20Data)))

(event Custom|ChangeServer
  (Variables|Default|SetServerToConnectTo (Utilities|Select :Index (Variables|Default|GetWebsocketServer) :NewEnumerator0 (Variables|Default|GetScanReachServer) :NewEnumerator1 (Variables|Default|GetScanReachEchoServer)))
  (Utilities|IsValid (Variables|Default|GetWebsocket)
    (:Is%20Valid
      (CallFunction|WebSocketDisconnect))
    (:Is%20Not%20Valid
      _))
  (CallFunction|ConnecttoServer))

(event Custom|WebSocketDisconnect
  (Class|WebSocketBase|Close (Variables|Default|GetWebsocket))
  (Variables|Default|SetWebsocket 0))

(event Custom|WebSocketConnectError
  (params (error :type String))
  (Development|PrintString error)
  (CallFunction|ConnecttoServer))

(event Custom|ConnectToServer
  (bind _returnvalue (Class|WebSocketBlueprintLibrary|Connect (Variables|Default|GetServerToConnectTo)))
  (bind _output_get (Variables|Default|SetWebsocket _returnvalue))
  (EventDispatchers|BindEventtoOnConnectComplete _output_get (delegate Custom|WebSocketConnected))
  (EventDispatchers|BindEventtoOnConnectError _output_get (delegate Custom|WebSocketConnectError))
  (Class|WebSocketBase|SendText _output_get "{\"Name\": \"Interval\", \"Value\": 1000}"))

(event Custom|SendDataToSensor
  (params (Sensor :type Bp%20Sensor%20Object%20Reference) (WebSocketPacket :type Websocket%20Test%20Object%20Reference) (TagID :type TESTMOVEMENT%20Object%20Reference))
  (Default|SearchandMoveTagId Sensor TagID))

(event Custom|WebSocketRecieve%20Data
  (params (data :type String))
  (bind _returnvalue (Class|WebSocketBlueprintLibrary|JsontoObject data "/Game/Blueprints/Websocket/WebsocketTest.WebsocketTest_C" false))
  (bind _output_get (Variables|Default|SetJsonObject _returnvalue))
  (bind _aswebsocket_test (Utilities|Casting|CastToWebsocketTest _output_get))
  (bind _data (Class|WebSocketBlueprintLibrary|ObjecttoJson _aswebsocket_test))
  (Development|PrintString _data)
  (if (Utilities|Array|ContainsItem (Variables|Default|GetTagID's) (Variables|/Game/Blueprints/Websocket/WebsocketTest.WebsocketTest_C|GetTagID _aswebsocket_test))
    (for _array_element (Variables|Default|GetAllTags)
      (if (Utilities|Enum|Equal(Enum) (Variables|/Game/Blueprints/Websocket/WebsocketTest.WebsocketTest_C|GetTagID _aswebsocket_test) (Variables|/Game/Blueprints/Ship/TESTMOVEMENT.TESTMOVEMENT_C|GetTagID _array_element))
        (Variables|Default|SetCurrentTagid _array_element)))
    (else
      (bind _returnvalue_2 (Game|SpawnActorfromClass "/Game/Blueprints/Ship/TESTMOVEMENT.TESTMOVEMENT_C" (Math|Transform|MakeTransform "0.000000, 0, 0" "0.000000, 0, 0" "1,1,1") "Undefined" 0 (Variables|Default|Getbp_ship) 0))
      (bind _output_get_2 (Variables|/Game/Blueprints/Ship/TESTMOVEMENT.TESTMOVEMENT_C|SetTagID _returnvalue_2 (Variables|/Game/Blueprints/Websocket/WebsocketTest.WebsocketTest_C|GetTagID _aswebsocket_test)))
      (Utilities|Array|AddUnique (Variables|Default|GetTagID's) _output_get_2)
      (Development|PrintString (Utilities|String|Append "New Pawn: " _output_get_2) true true "(R=0.010368,G=1.000000,B=0.000000,A=1.000000)")
      (bind _output_get_3 (Variables|Default|SetCurrentTagid _returnvalue_2))
      (Utilities|Array|AddUnique (Variables|Default|GetAllTags) _output_get_3)))
  (for _array_element_2 (Variables|Default|GetSensorList)
    (if (Utilities|Enum|Equal(Enum) (Variables|/Game/Blueprints/Ship/bp_Sensor.bp_Sensor_C|GetSensorID _array_element_2) (Variables|/Game/Blueprints/Websocket/WebsocketTest.WebsocketTest_C|GetSensorID _aswebsocket_test))
      (Variables|/Game/Blueprints/Ship/bp_Sensor.bp_Sensor_C|SetLastDataRecieved _array_element_2 _data)
      (CallFunction|SendDatatoSensor _array_element_2 _aswebsocket_test (Variables|Default|GetCurrentTagid)))))

(event Custom|ChangeMode)

(event EventBeginPlay
  (Utilities|FlowControl|Delay 0.5)
  (switch Utilities|FlowControl|Switch|SwitchonModeEnum (Variables|Default|GetModeEnum)
    (:NewEnumerator1
      (CallFunction|ConnecttoServer))))

(fn ConstructionScript)