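; Websocket manager Blueprint that streams tag signal readings (RSSI, TagID, SensorID) from a server into the level's Bp_Sensor actors.
; On BeginPlay it caches the sensors, connects, sends an interval setting, and reconnects on connection errors.
; Incoming JSON is parsed into Websocket_Sort, logged, recorded by unique tag, and routed to the sensor with the matching ID.
; ChangeServer switches the connection to ScanReachServer; ChangeMode is an empty stub.
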(event Custom|CallXData
  (params (Index :type Integer))
  (Development|PrintString (Utilities|Array|Get(acopy) (Variables|Default|GetLogOfDataStings) Index)))

(event Custom|WebSocketConnected
  (Development|PrintString (Utilities|String|Append "Connected To: " (Variables|Default|GetServerToConnectTo)))
  (Class|WebSocketBase|SendText (stale Custom|ConnectToServer _output_get) "{\"Name\": \"Interval\", \"Value\": 2000}")
  (EventDispatchers|AssignOnReceiveData (stale Custom|ConnectToServer _output_get) (delegate Custom|WebSocketRecieve%20Data)))

(event Custom|WebSocketRecieve%20Data
  (params (data :type String))
  (bind _returnvalue (Class|WebSocketBlueprintLibrary|JsontoObject data "/Game/Blueprints/Websocket/Websocket_Sort.Websocket_Sort_C" false))
  (bind _output_get (Variables|Default|SetJsonObject _returnvalue))
  (bind _aswebsocket_sort (Utilities|Casting|CastToWebsocket_Sort _output_get))
  (Utilities|FlowControl|Sequence
    (:then_0
      (bind _data (Class|WebSocketBlueprintLibrary|ObjecttoJson _aswebsocket_sort))
      (bind _output_get_2 (Variables|Default|SetLastDataRecieved _data))
      (Utilities|Array|Add (Variables|Default|GetLogOfDataStings) _output_get_2))
    (:then_1
      (CallFunction|UpdateTagID's (Variables|/Game/Blueprints/Websocket/Websocket_Sort.Websocket_Sort_C|GetTagID _aswebsocket_sort)))
    (:then_2
      (Development|PrintString (Utilities|String|Append (Utilities|String|Append "RSSI: " (Variables|/Game/Blueprints/Websocket/Websocket_Sort.Websocket_Sort_C|GetRSSI _aswebsocket_sort)) " 
 
" (Utilities|String|Append "TagID: " (Variables|/Game/Blueprints/Websocket/Websocket_Sort.Websocket_Sort_C|GetTagID _aswebsocket_sort)) " 
 
" (Utilities|String|Append "SensorID: " (Variables|/Game/Blueprints/Websocket/Websocket_Sort.Websocket_Sort_C|GetSensorID _aswebsocket_sort))))
      (CallFunction|CollectandSendData (Variables|/Game/Blueprints/Websocket/Websocket_Sort.Websocket_Sort_C|GetRSSI _aswebsocket_sort) (Variables|/Game/Blueprints/Websocket/Websocket_Sort.Websocket_Sort_C|GetTagID _aswebsocket_sort) (Variables|/Game/Blueprints/Websocket/Websocket_Sort.Websocket_Sort_C|GetSensorID _aswebsocket_sort)))))

(event Custom|ConnectToServer
  (bind _returnvalue (Class|WebSocketBlueprintLibrary|Connect (Variables|Default|GetServerToConnectTo)))
  (bind _output_get (Variables|Default|SetWebsocket _returnvalue))
  (EventDispatchers|BindEventtoOnConnectComplete _output_get (delegate Custom|WebSocketConnected))
  (EventDispatchers|BindEventtoOnConnectError _output_get (delegate Custom|WebSocketConnectError)))

(event Custom|WebSocketConnectError
  (params (error :type String))
  (Development|PrintString error)
  (CallFunction|ConnecttoServer))

(event Custom|WebSocketDisconnect
  ;[1 1 1] Disconnect current connection
  (Class|WebSocketBase|Close (Variables|Default|GetWebsocket))
  (Variables|Default|SetWebsocket 0))

(event Custom|ChangeMode)

(event Custom|ChangeServer
  ;[1 1 1] Call to change server
  (Variables|Default|SetServerToConnectTo (Variables|Default|GetScanReachServer))
  (Utilities|IsValid (Variables|Default|GetWebsocket)
    (:Is%20Valid
      (CallFunction|WebSocketDisconnect))
    (:Is%20Not%20Valid
      _))
  (CallFunction|ConnecttoServer))

(event EventBeginPlay
  (bind _outactors (Actor|GetAllActorsOfClass "/Game/Blueprints/Ship/bp_Sensor.bp_Sensor_C"))
  (for _array_element _outactors
    (Utilities|Array|AddUnique (Variables|Default|GetSensorID's) (Variables|/Game/Blueprints/Ship/bp_Sensor.bp_Sensor_C|GetSensorID _array_element))
    (Development|PrintString (Variables|/Game/Blueprints/Ship/bp_Sensor.bp_Sensor_C|GetSensorID _array_element))
    (Utilities|Array|AddUnique (Variables|Default|GetSensorRefs) _array_element))
  (Utilities|FlowControl|Delay 0.5)
  (CallFunction|ConnecttoServer))

(fn ConstructionScript)

(fn CollectandSendData
  (params (RSSI :type String) (TagID :type String) (SensorID :type String))
  (for _array_element (Variables|Default|GetSensorRefs)
    (if (Utilities|Enum|Equal(Enum) SensorID (Variables|/Game/Blueprints/Ship/bp_Sensor.bp_Sensor_C|GetSensorID _array_element))
      (LocalVariables|SetValidSensor _array_element)))
  (Default|UpdateInformation (LocalVariables|GetValidSensor) TagID "" "" "" "" RSSI))

(fn UpdateTagID's
  (params (TagId :type String))
  (if (not (Utilities|Array|ContainsItem (Variables|Default|GetAllTagId's) TagId))
    (Utilities|Array|AddUnique (Variables|Default|GetAllTagId's) TagId)))